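; BP_Leviathan is a VR throwable axe that motion controllers pick up, throw and recall to the hand.
; Pickup cancels recovery, registers the axe on the MotionControllerPawn and snaps it to the hand's Weapon socket with physics off.
; Drop detaches it and always calls ThrowAxe, as the hand-velocity threshold check is disconnected.
; A successful OnRecoverFinished re-attaches it to the stored hand.
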(event `/Game/VirtualRealityBP/Blueprints/PickupActorInterface.Pickup`
  (params (AttachTo :type "SceneComponent Object Reference"))
  (set `self.IsRecoverActive` false)
  (set `self.Actor` AttachTo)
  (bind _asmotion_controller_pawn (cast `/Game/VirtualRealityBP/Blueprints/MotionControllerPawn` (`self.GetOwner` (`ActorComponent.GetOwner` AttachTo))))
  (set `/Game/VirtualRealityBP/Blueprints/MotionControllerPawn.Axe` self _asmotion_controller_pawn)
  (bind _output_get (set `self.Hand` AttachTo))
  (`self.AttachToHand` _output_get))

(event `self.K2_OnRecoverFinished`
  (params (success :type Boolean))
  (if success
    (`self.AttachToHand` (`self.Hand`))))

(event `/Game/VirtualRealityBP/Blueprints/PickupActorInterface.Drop`
  (`self.K2_DetachFromActor` "KeepWorld" "KeepWorld" "KeepWorld")
  (bind _returnvalue (`PrimitiveComponent.GetPhysicsLinearVelocity` (`self.GetComponentByClass` (`ActorComponent.GetOwner` (`self.Actor`)) "/Script/Engine.SphereComponent") "None"))
  (`self.ThrowAxe`)
  (set `self.Actor` null))

(fn `AttachToHand`
  (params (Hand :type "SceneComponent Object Reference"))
  (bind _staticmesh (`self.StaticMesh`))
  (`PrimitiveComponent.SetSimulatePhysics` _staticmesh false)
  (`SceneComponent.K2_AttachToComponent` (`self.K2_GetRootComponent`) Hand "Weapon" "SnapToTarget" "SnapToTarget" "KeepRelative" true)
  (`SceneComponent.K2_SetRelativeLocation` _staticmesh (0.0 0.0 21.891474) false false))

(fn `UserConstructionScript`)